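; BP_TimerMenu is an actor that shows a W_Timer widget with a UXTools pressable button for picking a timer setting.
; On BeginPlay it caches the widget and binds to the child button actor's press event.
; A press broadcasts the OnSetTimer dispatcher with the widget's selected item, then destroys the menu actor.
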(event `self.ReceiveBeginPlay`
  (bind _asw_timer (cast `/Game/Widgets/W_Timer` (`WidgetComponent.GetWidget` (`self.Widget`))))
  (set `self.As W Timer` _asw_timer)
  (bind _asuxt_pressable_button_actor (cast `UxtPressableButtonActor` (`ChildActorComponent.ChildActor` (`self.ChildActor`))))
  (add `UxtPressableButtonComponent.OnButtonPressed` (`UxtBasePressableButtonActor.ButtonComponent` _asuxt_pressable_button_actor) (delegate `CustomEvent_0`)))

(event `CustomEvent_0`
  (params (Button :type "UxtPressableButtonComponent Object Reference") (Pointer :type "UxtPointerComponent Object Reference"))
  (`self.OnSetTimer` (`/Game/Widgets/W_Timer.Selected Item` (`self.As W Timer`)))
  (`self.K2_DestroyActor`))

(fn `UserConstructionScript`)