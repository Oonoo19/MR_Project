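; AC_Timer is a countdown timer component that takes a duration, multiplies it by 60 and counts down once per second.
; Starttimer stores the count, prints the raw duration and starts a looping function-name timer on UpdateTimer.
; UpdateTimer decrements the count, calling StopTimer at zero or below.
; StopTimer clears the timer handle and fires the OnStopTimer dispatcher, with an alarm marked only by a comment.
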(event `self.ReceiveBeginPlay`)

(event `Start timer`
  (params (Duration :type Integer))
  (set `self.Timer` (* Duration 60))
  (`KismetSystemLibrary.PrintString` (`KismetStringLibrary.Conv_IntToString` Duration))
  (bind _returnvalue (`KismetSystemLibrary.K2_SetTimer` null "UpdateTimer" 1.0 true)))

(event `StopTimer`
  (`KismetSystemLibrary.K2_ClearAndInvalidateTimerHandle` (stale `Start timer` _returnvalue))
  ;[1 1 1] Alarm here
  (`self.OnStopTimer`))

(fn `UpdateTimer`
  (`/Engine/EditorBlueprintResources/StandardMacros.CompareInt` (`self.Timer`)
    (:`>`
      (`/Engine/EditorBlueprintResources/StandardMacros.DecrementInt` (`self.Timer`)))
    (:`==`
      (`self.StopTimer` :!label _label))
    (:`<`
      (goto _label))))