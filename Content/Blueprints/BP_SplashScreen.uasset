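; Splash screen actor for a mixed-reality app, hosting a W_SplashScreen widget that leads from a start button into scanning.
; On BeginPlay it caches the widget and MRPawn and binds both widget callbacks.
; Start switches to the scanning view and begins scanning after a short delay; the actor destroys itself when the scanning widget signals destruction.
; An older UXT button path that starts a pawn session with a water-pattern material remains unwired.
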(event `self.ReceiveBeginPlay`
  (`|ExecutionSequence`
    (:`then_0`
      (bind _asw_splash_screen (cast `/Game/Widgets/W_SplashScreen` (`WidgetComponent.GetWidget` (`self.Widget`))))
      (set `self.As W Splash Screen` _asw_splash_screen)
      (bind _asmrpawn (cast `/Game/Blueprints/MRPawn` (`GameplayStatics.GetPlayerPawn` 0)))
      (set `self.As MRPawn` _asmrpawn)
      ;[0 0 0] Scanning
      (add `/Game/Widgets/W_SplashScreen.OnUIButtonPressed` (`self.As W Splash Screen`) (delegate `OnStartButtonPressed`))
      (add `/Game/Widgets/W_Scanning.OnDestroy` (`/Game/Widgets/W_SplashScreen.W_Scanning` (`self.As W Splash Screen`)) (delegate `OnScanningFinished`)))))

(event `OnStartButtonPressed`
  (bind _as_w_splash_screen (`self.As W Splash Screen`))
  ;[0 0 0] Scanning
  (`WidgetSwitcher.SetActiveWidgetIndex` (`/Game/Widgets/W_SplashScreen.Switcher` _as_w_splash_screen) 1)
  (`KismetSystemLibrary.Delay` 0.2)
  (`/Game/Widgets/W_Scanning.StartScanning` (`/Game/Widgets/W_SplashScreen.W_Scanning` _as_w_splash_screen)))

(event `OnScanningFinished`
  (`self.K2_DestroyActor` self))

(event `CustomEvent_0`
  (params (Button :type "UxtPressableButtonComponent Object Reference") (Pointer :type "UxtPointerComponent Object Reference"))
  (bind _returnvalue (`KismetMaterialLibrary.CreateDynamicMaterialInstance` "/Game/Materials/M_WaterPattern2.M_WaterPattern2"))
  (`/Game/Blueprints/MRPawn.StartSession` (`self.As MRPawn`) _returnvalue)
  (`UxtUIElementComponent.SetUIVisibility` (`self.UxtUIElement`) "Hide"))

(fn `UserConstructionScript`)