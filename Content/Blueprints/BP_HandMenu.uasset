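; Mixed reality hand menu using UX Tools, shown and hidden by a palm-up constraint.
; On BeginPlay it shows the first of three panels and binds music, end and timer buttons.
; These buttons drive the MRPawn's audio toggle, session end and timer.
; Navigate switches panels by visibility, but arrow bindings are disconnected, and going left from Menu3 lands on Menu1 instead of Menu2.
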(event `self.UxtPalmUpConstraint.OnConstraintActivated`
  (`UxtUIElementComponent.SetUIVisibility` (`self.UxtUIElement`) "Show"))

(event `self.UxtPalmUpConstraint.OnConstraintDeactivated`
  (`UxtUIElementComponent.SetUIVisibility` (`self.UxtUIElement`) "Hide"))

(event `self.ReceiveBeginPlay`
  (`|ExecutionSequence`
    (:`then_0`
      (bind _asmrpawn (cast `/Game/Blueprints/MRPawn` (`GameplayStatics.GetPlayerPawn` 0)))
      (set `self.As MRPawn` _asmrpawn)
      (bind _asuxt_pressable_switch_button_actor (cast `UxtPressableSwitchButtonActor` (`ChildActorComponent.ChildActor` (`self.MusicButton`))))
      (`UxtPressableButtonComponent.SetEnabled` (`UxtBasePressableButtonActor.ButtonComponent` _asuxt_pressable_switch_button_actor) true))
    (:`then_1`
      (`SceneComponent.SetVisibility` (`self.UxtUIElement`) true true)
      (`SceneComponent.SetVisibility` (`self.Menu1`) true true)
      (`SceneComponent.SetVisibility` (`self.Menu2`) false true)
      (`SceneComponent.SetVisibility` (`self.Menu3`) false true))
    (:`then_2`
      (bind _asuxt_pressable_switch_button_actor_2 (cast `UxtPressableSwitchButtonActor` (`ChildActorComponent.ChildActor` (`self.MusicButton`))))
      (add `UxtToggleStateComponent.OnToggled` (`UxtPressableToggleButtonActor.ToggleStateComponent` _asuxt_pressable_switch_button_actor_2) (delegate `CustomEvent_1`))
      (bind _asuxt_pressable_button_actor (cast `UxtPressableButtonActor` (`ChildActorComponent.ChildActor` (`self.End`))))
      (add `UxtPressableButtonComponent.OnButtonPressed` (`UxtBasePressableButtonActor.ButtonComponent` _asuxt_pressable_button_actor) (delegate `OnEndButtonPressed`))
      (bind _asuxt_pressable_button_actor_2 (cast `UxtPressableButtonActor` (`ChildActorComponent.ChildActor` (`self.TimerButton`))))
      (add `UxtPressableButtonComponent.OnButtonPressed` (`UxtBasePressableButtonActor.ButtonComponent` _asuxt_pressable_button_actor_2) (delegate `OnTimerButtonPressed`)))))

(event `OnButtonPressed_Event_0`
  (params (Button :type "UxtPressableButtonComponent Object Reference") (Pointer :type "UxtPointerComponent Object Reference"))
  ;[0 0 0] Navigate to right or left
  (`self.Navigate` false))

(event `OnButtonPressed_Event_1`
  (params (Button :type "UxtPressableButtonComponent Object Reference") (Pointer :type "UxtPointerComponent Object Reference"))
  ;[0 0 0] Navigate to right or left
  (`self.Navigate` true))

(event `CustomEvent_1`
  (params (ToggleState :type "UxtToggleStateComponent Object Reference"))
  (bind _audio (`/Game/Blueprints/MRPawn.Audio` (`self.As MRPawn`)))
  (if (`UxtToggleStateComponent.bIsChecked` ToggleState)
    (`/Game/Music/BP_Underwater.PlayAudio` _audio)
    (else
      (`/Game/Music/BP_Underwater.StopAudio` _audio))))

(event `OnEndButtonPressed`
  (params (Button :type "UxtPressableButtonComponent Object Reference") (Pointer :type "UxtPointerComponent Object Reference"))
  (`/Game/Blueprints/MRPawn.OnSessionEnd` (`self.As MRPawn`)))

(event `OnTimerButtonPressed`
  (params (Button :type "UxtPressableButtonComponent Object Reference") (Pointer :type "UxtPointerComponent Object Reference"))
  (`/Game/Blueprints/MRPawn.Timer` (`self.As MRPawn`)))

(event `Navigate`
  (params (ToRight :type Boolean))
  ;[0 0 0] Navigation visibility toggle
  (if ToRight
    (if (`SceneComponent.IsVisible` (`self.Menu1`))
      (`SceneComponent.SetVisibility` (`self.Menu1`) false true)
      (`SceneComponent.SetVisibility` (`self.Menu2`) true true)
      (elif (`SceneComponent.IsVisible` (`self.Menu2`))
        (`SceneComponent.SetVisibility` (`self.Menu2`) false true)
        (`SceneComponent.SetVisibility` (`self.Menu3`) true true)
        (elif (`SceneComponent.IsVisible` (`self.Menu3`))
          (`SceneComponent.SetVisibility` (`self.Menu3`) false true)
          (`SceneComponent.SetVisibility` (`self.Menu1`) true true))))
    (elif (`SceneComponent.IsVisible` (`self.Menu1`))
      (`SceneComponent.SetVisibility` (`self.Menu1`) false true)
      (`SceneComponent.SetVisibility` (`self.Menu3`) true true)
      (elif (`SceneComponent.IsVisible` (`self.Menu2`))
        (`SceneComponent.SetVisibility` (`self.Menu2`) false true)
        (`SceneComponent.SetVisibility` (`self.Menu1`) true true)
        (elif (`SceneComponent.IsVisible` (`self.Menu3`))
          (`SceneComponent.SetVisibility` (`self.Menu3`) false true)
          (`SceneComponent.SetVisibility` (`self.Menu1`) true true))))))

(fn `UserConstructionScript`)