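; Mixed reality pawn that hosts an underwater-themed timed session, spawning UXT hands, the splash screen, an underwater actor and menus.
; Spatial mapping capture retries on a timer until enabled, then world meshes receive a water material as they are added or updated.
; The timer menu feeds the chosen time to ACTimer, whose stop event spawns the end widget.
; StartSession applies a given material to the splash screen's tracked geometry.
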(event `Timer`
  (bind (_returnvalue_location _returnvalue_rotation _returnvalue_scale) (`KismetMathLibrary.BreakTransform` (`self.GetTransform` self)))
  (`/Engine/EditorBlueprintResources/StandardMacros.IsValid` (`self.BP_Timer`)
    (:`Is Not Valid`
      (bind _returnvalue (`|SpawnActorFromClass` "/Game/Blueprints/BP_TimerMenu.BP_TimerMenu_C" (`KismetMathLibrary.MakeTransform` (`KismetMathLibrary.MakeVector` (+ (.x _returnvalue_location) 40.0) (.y _returnvalue_location) (.z _returnvalue_location)) _returnvalue_rotation _returnvalue_scale) "Undefined" "OverrideRootScale" null null))
      (bind _output_get (set `self.BP_Timer` _returnvalue))
      (add `/Game/Blueprints/BP_TimerMenu.OnSetTimer` _output_get (delegate `CustomEvent_0`)))))

(event `CustomEvent_0`
  (params (Time :type "Float (double-precision)"))
  (`/Game/Blueprints/AC_Timer.Start timer` (`self.AC_Timer`) (`KismetMathLibrary.FTrunc` Time)))

(event `self.ReceiveBeginPlay`
  (`self.SpawnUI`)
  (`self.SpawnVirtualHands`)
  (`self.UnderwaterMapping`)
  (add `/Game/Blueprints/AC_Timer.OnStopTimer` (`self.AC_Timer`) (delegate `OnStopTimer_Event_0`))
  (`self.EnabledSpatialMappingRecurse`))

(event `OnStopTimer_Event_0`
  (`self.OnSessionEnd`))

(event `UnderwaterMapping`
  (bind _returnvalue (`|SpawnActorFromClass` "/Game/Music/BP_Underwater.BP_Underwater_C" (`KismetMathLibrary.MakeTransform` (0.0 0.0 0.0)) "Undefined" "OverrideRootScale" null null))
  (set `self.Audio` _returnvalue))

(event `OnSessionEnd`
  (bind (_returnvalue_location _returnvalue_rotation _returnvalue_scale) (`KismetMathLibrary.BreakTransform` (`self.GetTransform` self)))
  ;[0 0 0] Spawn End Widget
  (`/Engine/EditorBlueprintResources/StandardMacros.IsValid` (`self.EndWidget`)
    (:`Is Not Valid`
      (bind _returnvalue (`|SpawnActorFromClass` "/Game/Blueprints/BP_End.BP_End_C" (`KismetMathLibrary.MakeTransform` (`KismetMathLibrary.MakeVector` (+ (.x _returnvalue_location) 50.0) (.y _returnvalue_location) (.z _returnvalue_location)) _returnvalue_rotation _returnvalue_scale) "Undefined" "OverrideRootScale" self null))
      (set `self.EndWidget` _returnvalue)
      (`self.OnQuit`))))

(event `SpawnVirtualHands`
  (bind _returnvalue (`KismetMathLibrary.MakeTransform` (0.0 0.0 0.0)))
  ;[0 0 0] Spawn Virtual Hands
  (`|SpawnActorFromClass` "/Script/UXTools.UxtHandInteractionActor" _returnvalue "Undefined" "OverrideRootScale" null false "Left" self)
  (`|SpawnActorFromClass` "/Script/UXTools.UxtHandInteractionActor" _returnvalue "Undefined" "OverrideRootScale" null false "Right" self))

(event `self.ReceiveEndPlay`
  (params (EndPlayReason :type "EEndPlayReason Enum" :default "Destroyed"))
  (`ARBlueprintLibrary.ToggleARCapture` false "SpatialMapping"))

(event `SpawnUI`
  (bind (_returnvalue_location _returnvalue_rotation _returnvalue_scale) (`KismetMathLibrary.BreakTransform` (`self.GetTransform` self)))
  ;[0 0 0] Spawn UI
  (bind _returnvalue (`|SpawnActorFromClass` "/Game/Blueprints/BP_SplashScreen.BP_SplashScreen_C" (`KismetMathLibrary.MakeTransform` (`KismetMathLibrary.MakeVector` (+ (.x _returnvalue_location) 40.0) (.y _returnvalue_location) (.z _returnvalue_location)) _returnvalue_rotation _returnvalue_scale) "Undefined" "OverrideRootScale" self null))
  (set `self.SplashScreen` _returnvalue))

(event `StartSession`
  (params (Material :type "MaterialInstanceDynamic Object Reference"))
  ;[0 0 0] Start Mapping Material
  (for _array_element (`/Game/Blueprints/BP_SplashScreen.Tracked Geometry` (`self.SplashScreen`))
    (`/Engine/EditorBlueprintResources/StandardMacros.IsValid` _array_element
      (:`Is Valid`
        (`PrimitiveComponent.SetMaterial` (`ARTrackedGeometry.GetUnderlyingMesh` _array_element) 0 Material))
      (:`Is Not Valid`
        (`KismetSystemLibrary.PrintString` "motttttttttttttttttttt")))))

(event `self.ARTrackableNotify.OnAddTrackedGeometry`
  (params (TrackedGeometry :type "ARTrackedGeometry Object Reference"))
  (bind _returnvalue (`ARTrackedGeometry.GetUnderlyingMesh` TrackedGeometry))
  ;[0 0 0] Spatial mapping
  (if (and (`|EnumEquality` (`ARTrackedGeometry.GetObjectClassification` TrackedGeometry) "World") (`KismetSystemLibrary.IsValid` _returnvalue))
    ;;[0 0 0] Only adding new elements to array
    (`KismetArrayLibrary.Array_AddUnique` (`self.TrackedGeometry`) _returnvalue)
    (`PrimitiveComponent.SetMaterial` _returnvalue 0 "/Game/Materials/M_WaterPattern2.M_WaterPattern2")))

(event `self.ARTrackableNotify.OnUpdateTrackedGeometry`
  (params (TrackedGeometry :type "ARTrackedGeometry Object Reference"))
  (bind _returnvalue (`ARTrackedGeometry.GetUnderlyingMesh` TrackedGeometry))
  ;[0 0 0] Spatial mapping
  (if (and (`|EnumEquality` (`ARTrackedGeometry.GetObjectClassification` TrackedGeometry) "World") (`KismetSystemLibrary.IsValid` _returnvalue))
    ;;[0 0 0] Only adding new elements to array
    (`KismetArrayLibrary.Array_AddUnique` (`self.TrackedGeometry`) _returnvalue)
    (`PrimitiveComponent.SetMaterial` _returnvalue 0 "/Game/Materials/M_WaterPattern2.M_WaterPattern2")))

(event `ToggleARSession`
  (params (Active :type Boolean))
  ;[0 0 0] Spatial mapping
  (if Active
    (`ARBlueprintLibrary.StartARSession` null)
    (else
      (`ARBlueprintLibrary.PauseARSession`))))

(event `InputAction|OpenNearMenu`
  (params (Key :type "Key Structure"))
  ;[0 0 0] Spawn Near Menu
  (:`Pressed`
    (`|SpawnActorFromClass` "/Game/Blueprints/BP_NearMenu.BP_NearMenu_C" (`KismetMathLibrary.MakeTransform` (50.0 0.0 0.0)) "Undefined" "OverrideRootScale" self null)))

(fn `EnabledSpatialMappingRecurse`
  (`KismetSystemLibrary.PrintString` "Hello")
  (bind _returnvalue (`ARBlueprintLibrary.ToggleARCapture` true "SpatialMapping"))
  ;[0 0 0] Keep enabling until it is successful.
  (if _returnvalue
    (`KismetSystemLibrary.PrintString` "enabled")
    (else
      (`KismetSystemLibrary.K2_SetTimer` null "EnabledSpatialMappingRecurse" 0.2))))

(fn `UserConstructionScript`)