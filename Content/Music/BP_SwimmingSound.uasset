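; BP_SwimmingSound plays a looping swimming sound, judging by its name, through an audio component.
; BeginPlay starts playback and binds the component's audio-finished event to a handler that replays it from the start, looping it in Blueprint.
; PlayAudio and StopAudio events start or stop the component, each checking whether it is already playing.
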(event `self.ReceiveBeginPlay`
  (bind _audiocomponent (`self.AudioComponent`))
  (`AudioComponent.Play` _audiocomponent 0.0)
  (add `AudioComponent.OnAudioFinished` _audiocomponent (delegate `OnFinished`)))

(event `OnFinished`
  (`AudioComponent.Play` (`self.AudioComponent`) 0.0))

(event `StopAudio`
  (if (`AudioComponent.IsPlaying` (`self.AudioComponent`))
    (`AudioComponent.Stop` (`self.AudioComponent`))))

(event `PlayAudio`
  (if (not (`AudioComponent.IsPlaying` (`self.AudioComponent`)))
    (`AudioComponent.Play` (`self.AudioComponent`) 0.0)))

(fn `UserConstructionScript`)